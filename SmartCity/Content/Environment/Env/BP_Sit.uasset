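; BP_Sit is an interactable bus stop prop that lets the interacting character sit down and stand back up.
; StartInteraction disables the prop's collision, plays a stand-to-sit montage and eases the character's root to a hardcoded offset from the actor using MoveComponentTo.
; EndInteraction plays the sit-to-stand montage, stops the sitting montage, then after a delay restores collision and re-enables movement.
; The call that would disable movement is unconnected.
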(event EventBeginPlay
  (|CallParentFunction) ; This node is disabled and will not be called.\nDrag off pins to build functionality.
)

(event Collision|EventActorBeginOverlap
  (params (OtherActor :type Actor%20Object%20Reference))
  (|CallParentFunction OtherActor) ; This node is disabled and will not be called.\nDrag off pins to build functionality.
)

(event EventTick
  (params (DeltaSeconds :type Float%20%28single-precision%29))
  (|CallParentFunction DeltaSeconds) ; This node is disabled and will not be called.\nDrag off pins to build functionality.
)

(event EventStartInteraction
  (bind _returnvalue (Transformation|GetActorRotation))
  (bind _returnvalue_2 (Transformation|GetActorLocation))
  (Collision|SetCollisionEnabled (Variables|Default|Getprop_busstop_04) "NoCollision")
  (|CallParentFunction)
  (bind _ascharacter (Utilities|Casting|CastToCharacter (Variables|Default|GetInteractingActor)))
  (bind _output_get (Variables|Default|SetCharacter _ascharacter))
  (Animation|PlayAnimMontage _output_get "/Game/Characters/Mannequins/Animations/Manny/StandToSit_UE5_Montage.StandToSit_UE5_Montage" 1.0 "None")
  (Components|MoveComponentTo (Variables|/Script/Engine.Actor|GetRootComponent (Variables|Default|GetCharacter)) (Math|Vector|MakeVector (+ (.x _returnvalue_2) -1e+01) (+ (.y _returnvalue_2) 1e+02) (+ (.z _returnvalue_2) 105.0)) (Math|Rotator|MakeRotator (.roll _returnvalue) (.pitch _returnvalue) 9e+01) true true 0.5 false))

(event EventEndInteraction
  (|CallParentFunction)
  (bind _character (Variables|Default|GetCharacter)
    (:then
      (Animation|PlayAnimMontage _character "/Game/Characters/Mannequins/Animations/Manny/SitToStand_UE_Montage.SitToStand_UE_Montage" 1.0 "None")
      (Animation|StopAnimMontage _character "/Game/Characters/Mannequins/Animations/Manny/Sitting_3__UE5_Montage.Sitting_3__UE5_Montage")
      (Utilities|FlowControl|Delay 2.1)
      (Collision|SetCollisionEnabled (Variables|Default|Getprop_busstop_04) "QueryAndPhysics")
      (Class|BPICharacter|ToggleMovement(Message) (Variables|Default|GetCharacter) true))
    (:else)))

(fn ConstructionScript
  (|CallParentFunction))