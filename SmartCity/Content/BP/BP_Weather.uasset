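; Weather controller actor that blends the sky between clear and dark overcast and runs random, repeating rain cycles when rain is enabled.
; SetAtmosphereValues drives Rayleigh scattering on the sky atmosphere, post-process exposure compensation and a dynamic cloud material's density offset.
; Tick eases these toward target values at constant speed, disabling itself once exposure nears its target.
; StartRain darkens the sky, toggles the Raining reference on and off, clears, then randomly restarts.
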(event Custom|Dark
  (CallFunction|SetAtmosphereValues "(R=0.130136,G=0.149960,B=0.165132,A=1.000000)" -1.0 0.5))

(event Custom|Clear
  (CallFunction|SetAtmosphereValues "(R=0.174647,G=0.407240,B=1.000000,A=1.000000)" 1.0 0.0))

(event Custom|SetAtmosphereTargetParams
  (params (Target%20Cloud%20Density%20Offset :type Float%20%28single-precision%29) (Target%20Exposure%20Compensation :type Float%20%28single-precision%29) (Target%20Ray%20Leight%20Scatter :type Linear%20Color%20Structure))
  (Variables|AtmosphereValue|SetTarget%20Cloud%20Density%20Offset Target%20Cloud%20Density%20Offset)
  (Variables|AtmosphereValue|SetTarget%20Exposure%20Compensation Target%20Exposure%20Compensation)
  (Variables|AtmosphereValue|SetTarget%20Ray%20Leight%20Scatter Target%20Ray%20Leight%20Scatter)
  (Actor|Tick|SetActorTickEnabled true))

(event Custom|ToggleRain)

(event EventBeginPlay
  (Default|ToggleRain (Variables|Default|GetRaining) false)
  (if (Variables|Default|GetRain%20Enabled)
    (CallFunction|StartRain)))

(event Collision|EventActorBeginOverlap
  (params (OtherActor :type Actor%20Object%20Reference)))

(event EventTick
  (params (DeltaSeconds :type Float%20%28single-precision%29))
  (bind _returnvalue (Math|Float|MakeLiteralFloat 0.05))
  (bind _exposure_compensation (Variables|AtmosphereValue|GetExposure%20Compensation))
  (bind _target_exposure_compensation (Variables|AtmosphereValue|GetTarget%20Exposure%20Compensation))
  (CallFunction|SetAtmosphereValues (CallFunction|ColorInterptoConst (Variables|AtmosphereValue|GetRay%20Leight%20Scatter) (Variables|AtmosphereValue|GetTarget%20Ray%20Leight%20Scatter) _returnvalue) (Math|Interpolation|FInterptoConstant _exposure_compensation _target_exposure_compensation DeltaSeconds _returnvalue) (Math|Interpolation|FInterptoConstant (Variables|AtmosphereValue|GetCloud%20Density%20Offset) (Variables|AtmosphereValue|GetTarget%20Cloud%20Density%20Offset) DeltaSeconds _returnvalue))
  (Actor|Tick|SetActorTickEnabled (not (Math|Float|NearlyEqual(Float) _exposure_compensation _target_exposure_compensation 0.05))))

(fn ConstructionScript)

(fn SetAtmosphereValues
  (params (RayLeightScatter :type Linear%20Color%20Structure) (Exposure%20Compensation :type Float%20%28single-precision%29) (CloudDensityOffset :type Float%20%28single-precision%29))
  (Variables|AtmosphereValue|SetCloud%20Density%20Offset CloudDensityOffset)
  (Variables|AtmosphereValue|SetExposure%20Compensation Exposure%20Compensation)
  (Variables|AtmosphereValue|SetRay%20Leight%20Scatter RayLeightScatter)
  (bind _skyatmosphere (Variables|Default|GetSkyAtmosphere)
    (:then
      (Class|SkyAtmosphereComponent|SetRayleighScattering (Variables|/Script/Engine.SkyAtmosphere|GetSkyAtmosphereComponent _skyatmosphere) RayLeightScatter))
    (:else
      (Development|PrintString "Assign SkyAtmosphere Value")))
  (bind _postprocessvolume (Variables|Default|GetPostProcessVolume)
    (:then
      (Utilities|Struct|SetmembersinPostProcessSettings (Variables|/Script/Engine.PostProcessVolume|GetSettings _postprocessvolume) Exposure%20Compensation))
    (:else
      (Development|PrintString "Assign PostProcess volume")))
  (bind _volumetriccloud (Variables|Default|GetVolumetricCloud)
    (:then
      (Variables|Default|GetCloudMat
        (:then
          _)
        (:else
          (bind _returnvalue (Rendering|Material|CreateDynamicMaterialInstance "/Game/Environment/Cloud/m_SimpleVolumetricCloud_Inst.m_SimpleVolumetricCloud_Inst" "MClouds" "None" :!class /Script/Engine.KismetMaterialLibrary))
          (Variables|Default|SetCloudMat _returnvalue)))
      (Rendering|Material|SetMaterial (Variables|/Script/Engine.VolumetricCloud|GetVolumetricCloudComponent _volumetriccloud) (Variables|Default|GetCloudMat))
      (Rendering|Material|SetScalarParameterValue (Variables|Default|GetCloudMat) "Density Offset" CloudDensityOffset :!class /Script/Engine.MaterialInstanceDynamic))
    (:else
      (Development|PrintString "Assign Volumetric Cloud"))))

(fn ColorInterptoConst
  (params (InColor :type Linear%20Color%20Structure) (InColor2 :type Linear%20Color%20Structure) (InputPin :type Float%20%28double-precision%29))
  (bind _returnvalue (Utilities|Time|GetWorldDeltaSeconds))
  (bind (_r _g _b _a) (Math|Color|BreakColor InColor2))
  (bind (_r_2 _g_2 _b_2 _a_2) (Math|Color|BreakColor InColor))
  (return (Utilities|Struct|MakeLinearColor (Math|Interpolation|FInterptoConstant _r_2 _r _returnvalue InputPin) (Math|Interpolation|FInterptoConstant _g_2 _g _returnvalue InputPin) (Math|Interpolation|FInterptoConstant _b_2 _b _returnvalue InputPin) (Math|Interpolation|FInterptoConstant _a_2 _a _returnvalue InputPin))))

(event Custom|StartRain
  (Utilities|FlowControl|Delay 2.0)
  (CallFunction|SetAtmosphereTargetParams 0.5 -1.0 "(R=0.130136,G=0.149960,B=0.165132,A=1.000000)")
  (Utilities|FlowControl|Delay 3e+01)
  (bind _raining (Variables|Default|GetRaining)
    (:then
      (Default|ToggleRain _raining true)
      (Utilities|FlowControl|Delay 6e+01)
      (Default|ToggleRain (Variables|Default|GetRaining) false)
      (Utilities|FlowControl|Delay 5.0)
      (CallFunction|SetAtmosphereTargetParams 0.0 1.0 "(R=0.174647,G=0.407240,B=1.000000,A=1.000000)")
      (Utilities|FlowControl|Delay (Math|Random|RandomFloatinRange 3e+01 1.2e+02) :!label _label)
      (if (Math|Random|RandomBool)
        (CallFunction|StartRain)
        (else
          (goto _label))))
    (:else)))